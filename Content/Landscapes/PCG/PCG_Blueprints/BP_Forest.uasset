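; BP_Forest is a PCG landscape Blueprint that exposes on/off switches for the vegetation and ground-detail layers of a forest.
; The construction script turns each Enable flag into a full or zero density variable, covering trees, undergrowth, grass, rocks and shore foliage.
; The path toggle drives pebble density.
; The event graph is empty, and no scattering logic or reader of these densities appears in the Blueprint's graphs.
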(event EventBeginPlay)

(event Collision|EventActorBeginOverlap
  (params (OtherActor :type Actor%20Object%20Reference)))

(event EventTick
  (params (DeltaSeconds :type Float%20%28single-precision%29)))

(fn ConstructionScript
  (Variables|Default|SetDetailPlantDensity (select (Variables|Default|GetEnable_Detail_Plants) 1.0 0.0))
  (Variables|Default|SetShrubDensity (select (Variables|Default|GetEnable_Shrubs) 1.0 0.0))
  (Variables|Default|SetGrassDensity (select (Variables|Default|GetEnable_Grass) 1.0 0.0))
  (Variables|Default|SetPebbleDensity (select (Variables|Default|GetEnable_Path) 1.0 0.0))
  (Variables|Default|SetTreeDensity (select (Variables|Default|GetEnable_Trees) 1.0 0.0))
  (Variables|Default|SetShoreShrubsDensity (select (Variables|Default|GetEnable_ShoreFoliage) 1.0 0.0))
  (Variables|Default|SetRockDensity (select (Variables|Default|GetEnable_Rocks) 1.0 0.0))
  (Variables|Default|SetBushDensity (select (Variables|Default|GetEnable_Bushes) 1.0 0.0)))